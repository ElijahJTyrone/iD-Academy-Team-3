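; A moving platform actor template that oscillates back and forth around the position where it starts.
; BeginPlay stores the start location and packs speed, distance and an orientation flag into one vector.
; Each Tick adds speed to a counter and sets the location from its scaled sine, along Z when vertical or Y when horizontal.
; The counter advances per frame without delta time, so movement depends on frame rate.
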(event `self.ReceiveBeginPlay`
  ;[1 1 1] movingPlatform
  (set `self.startingPosition` (`self.K2_GetActorLocation`))
  (set `self.platformGeneral` (`KismetMathLibrary.MakeVector` (`self.speedOfPlatform`) (`self.distanceOfPlatform`) (`KismetMathLibrary.Conv_BoolToDouble` (`self.Orientation(False = Horizontal, True = Vertical)`)))))

(event `self.ReceiveTick`
  (params (DeltaSeconds :type "Float (single-precision)"))
  (bind (_startingposition_x _startingposition_y _startingposition_z) (`KismetMathLibrary.BreakVector` (`self.startingPosition`)))
  (bind (_platformgeneral_x _platformgeneral_y _platformgeneral_z) (`KismetMathLibrary.BreakVector` (`self.platformGeneral`)))
  (bind _returnvalue (+ _platformgeneral_x (`self.platformPositionCounter`)))
  (bind _returnvalue_2 (* (`KismetMathLibrary.Sin` _returnvalue) _platformgeneral_y))
  ;[1 1 1] movingPlatform
  (set `self.platformPositionCounter` _returnvalue)
  (if (`KismetMathLibrary.Conv_IntToBool` (`KismetMathLibrary.FTrunc` _platformgeneral_z))
    (`self.K2_SetActorLocation` (`KismetMathLibrary.MakeVector` _startingposition_x _startingposition_y (+ _returnvalue_2 _startingposition_z)))
    (else
      (`self.K2_SetActorLocation` (`KismetMathLibrary.MakeVector` _startingposition_x (+ _startingposition_y _returnvalue_2) _startingposition_z)))))

(fn `UserConstructionScript`)